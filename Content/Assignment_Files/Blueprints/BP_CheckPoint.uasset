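; BP_CheckPoint is a checkpoint actor with a looping bob and pulse animation, and it contains no trigger or save logic.
; BeginPlay caches the spawn location and scale as the base values.
; Tick accumulates time and uses the absolute sine of time and speed to lerp motion and scale offsets from zero, adding them to those base values.
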(event `self.ReceiveBeginPlay`
  (set `self.spawnLoaction` (`self.K2_GetActorLocation`))
  (set `self.spawnScale` (`self.GetActorScale3D`)))

(event `self.ReceiveTick`
  (params (DeltaSeconds :type "Float (single-precision)"))
  (bind _output_get (set `self.time` (+ DeltaSeconds (`self.time`))))
  (bind _returnvalue (`KismetMathLibrary.Abs` (`KismetMathLibrary.Sin` (* _output_get (`self.aniamtionSpeed`)))))
  (`self.K2_SetActorLocation` (+ (`KismetMathLibrary.VLerp` (0.0 0.0 0.0) (`self.animatedMotionAmont`) _returnvalue) (`self.spawnLoaction`)))
  (`self.SetActorScale3D` (+ (`KismetMathLibrary.VLerp` (0.0 0.0 0.0) (`self.animatedScaleAmount`) _returnvalue) (`self.spawnScale`))))

(fn `UserConstructionScript`)