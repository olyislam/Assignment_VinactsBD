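; Notifier component that shows title and message notifications on an on-screen UI canvas.
; On BeginPlay it creates a Main_Canvas widget, stores the instance and adds it to the viewport.
; SendGUINotification writes the given title and message into that widget's text fields, or prints a cancellation warning if the canvas reference is not yet set.
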(event `self.ReceiveBeginPlay`
  (bind _returnvalue (`|CreateWidget` "/Game/Assignment_Files/Widgets/Main_Canvas.Main_Canvas_C"))
  (bind _output_get (set `self.canvas_Instance` _returnvalue))
  (`UserWidget.AddToViewport` _output_get 0))

(fn `SendGUINotification`
  (params (title :type String) (message :type String))
  (bind _canvas_instance (`self.canvas_Instance`))
  (if (== _canvas_instance null)
    (`KismetSystemLibrary.PrintString` "Notifier Not Initialized Yet!!! [Notification Request Cancelled]")
    (else
      (`TextBlock.SetText` (`/Game/Assignment_Files/Widgets/Main_Canvas.Title_Text` _canvas_instance) (`KismetTextLibrary.Conv_StringToText` title))
      (`TextBlock.SetText` (`/Game/Assignment_Files/Widgets/Main_Canvas.Message_Txt` _canvas_instance) (`KismetTextLibrary.Conv_StringToText` message)))))